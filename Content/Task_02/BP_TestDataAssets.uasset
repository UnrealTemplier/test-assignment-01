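; BP_TestDataAssets is a test Blueprint that checks nested references between two data assets, DA1 and DA2.
; On BeginPlay it validates DA1, then DA2, printing a message for each.
; It then prints TestStructure's Name reached from DA2 into DA1, and through the circular chain DA1 to DA2 and back to DA1.
; Only the two top-level assets are validity-checked, not the nested references.
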(event EventBeginPlay
  (Variables|Default|GetDA_1
    (:then
      (Development|PrintString "DA_1 is valid!" true true "(R=0.000000,G=1.000000,B=0.136808,A=1.000000)" 1e+03)
      (Variables|Default|GetDA_2
        (:then
          (Development|PrintString "DA_2 is valid!" true true "(R=0.000000,G=1.000000,B=0.136808,A=1.000000)" 1e+03)
          (Development|PrintString (Utilities|String|Append "TestStructure's Name from DA_2->DA_1: " (.name (Variables|/Script/Redruins_TT_2024.DA_1|GetTestStructure (Variables|/Script/Redruins_TT_2024.DA_2|GetDataAsset1 (Variables|Default|GetDA_2))))) true true "(R=0.000000,G=1.000000,B=0.136808,A=1.000000)" 1e+03)
          (Development|PrintString (Utilities|String|Append "TestStructure's Name from DA_1->DA_2->DA_1: " (.name (Variables|/Script/Redruins_TT_2024.DA_1|GetTestStructure (Variables|/Script/Redruins_TT_2024.DA_2|GetDataAsset1 (.dataasset1 (Variables|/Script/Redruins_TT_2024.DA_1|GetTestStructure (Variables|Default|GetDA_1))))))) true true "(R=0.000000,G=1.000000,B=0.136808,A=1.000000)" 1e+03))
        (:else)))
    (:else)))

(fn ConstructionScript)