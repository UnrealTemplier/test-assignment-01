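; BP_Task_01_Character is a character Blueprint that lets the player interact with objects in front of the camera.
; On the IA_Interact input, it runs a Visibility line trace between points supplied by two helper functions, based on camera location, forward vector and InteractionDistance.
; If the hit actor implements BPI_Interactable, it sends InteractMessage through that interface, keeping the character decoupled from specific interactable classes.
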(event Input|EnhancedActionEvents|EnhancedInputActionIA_Interact
  (params (ActionValue :type Boolean) (ElapsedSeconds :type Float%20%28double-precision%29) (TriggeredSeconds :type Float%20%28double-precision%29) (InputAction :type Input%20Action%20Object%20Reference :default "/Game/Task_01/Input/IA_Interact.IA_Interact"))
  ;[1 1 1] Call Interact if it's possible
  (bind _outhit (Collision|LineTraceByChannel (Utilities|GetLineTraceStartPoint) (Utilities|GetLineTraceEndPoint) "TraceTypeQuery1" false 0 "None"))
  (if (Utilities|DoesObjectImplementInterface (.hitactor _outhit) "/Game/Task_01/Blueprints/BPI_Interactable.BPI_Interactable_C")
    (Class|BPIInteractable|Interact(Message) (.hitactor _outhit))))

(fn ConstructionScript)