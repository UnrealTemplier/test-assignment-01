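; BP_Task_01_Actor is a one-time interactable that swaps its sphere's material when used through BPI_Interactable.
; On BeginPlay it creates a W_Marker viewport widget linked to itself.
; Player overlap with SphereCollision runs a looping timer that toggles the interact widget.
; IsInteractable gates both prompt and interaction on proximity, unused state, line of sight and a camera trace hitting any BPI_Interactable actor.
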(event OnComponentBeginOverlap(SphereCollision)
  (params (OverlappedComponent :type Primitive%20Component%20Object%20Reference) (OtherActor :type Actor%20Object%20Reference) (OtherComp :type Primitive%20Component%20Object%20Reference) (OtherBodyIndex :type Integer) (bFromSweep :type Boolean) (SweepResult :type Hit%20Result%20Structure%20%28by%20ref%29))
  ;[1 1 1] Check if Player is near and Toggle widget visibility accordingly
  (if (Utilities|DoesObjectImplementInterface OtherActor "/Game/Task_01/Blueprints/BPI_Player.BPI_Player_C")
    (Variables|Default|SetPlayerIsNear true)
    (bind _returnvalue (Utilities|Time|SetTimerbyEvent (delegate Custom|ToggleWidget) 0.1 true))
    (Variables|Default|SetWidgetVisibilityTimer _returnvalue)))

(event OnComponentEndOverlap(SphereCollision)
  (params (OverlappedComponent :type Primitive%20Component%20Object%20Reference) (OtherActor :type Actor%20Object%20Reference) (OtherComp :type Primitive%20Component%20Object%20Reference) (OtherBodyIndex :type Integer))
  ;[1 1 1] Check if Player is near and Toggle widget visibility accordingly
  (if (Utilities|DoesObjectImplementInterface OtherActor "/Game/Task_01/Blueprints/BPI_Player.BPI_Player_C")
    (Variables|Default|SetPlayerIsNear false)
    (Utilities|Time|ClearandInvalidateTimerbyHandle (Variables|Default|GetWidgetVisibilityTimer))
    (Rendering|SetVisibility (Variables|Default|GetWidgetInteract) false false)))

(event Custom|ToggleWidget
  ;[1 1 1] Check if Player is near and Toggle widget visibility accordingly
  (Rendering|SetVisibility (Variables|Default|GetWidgetInteract) (CallFunction|IsInteractable) false))

(event EventInteract
  ;[1 1 1] BPI_Interactable implementation
  (if (CallFunction|IsInteractable)
    (CallFunction|ChangeMaterial)
    (Variables|Default|SetIsAlreadyInteracted true)))

(event EventBeginPlay
  ;[1 1 1] Initialization
  (bind _output_get (Variables|Default|SetPlayerControllerRef (Game|GetPlayerController 0)))
  (bind _returnvalue (UserInterface|CreateWidget "/Game/Task_01/Widgets/W_Marker.W_Marker_C" _output_get))
  (bind _output_get_2 (Variables|Default|SetWidgetMarker _returnvalue))
  (Variables|/Game/Task_01/Widgets/W_Marker.W_Marker_C|SetParentActor _output_get_2 self)
  (UserInterface|Viewport|AddtoViewport (Variables|Default|GetWidgetMarker) 0))

(fn ConstructionScript)

(fn ChangeMaterial
  (Rendering|Material|SetMaterial (Variables|Default|GetSphere) 0 "/Engine/MapTemplates/Materials/BasicAsset01.BasicAsset01"))

(fn IsInteractable
  (bind _outhit (Collision|LineTraceByChannel (Utilities|GetLineTraceStartPoint) (Utilities|GetLineTraceEndPoint) "TraceTypeQuery1" false 0 "None" false))
  (return (Math|Boolean|ANDBoolean (not (Variables|Default|GetIsAlreadyInteracted)) (Variables|Default|GetPlayerIsNear) (Controller|LineOfSightTo (Variables|Default|GetPlayerControllerRef) self "0, 0, 0" false) (Utilities|DoesObjectImplementInterface (.hitactor _outhit) "/Game/Task_01/Blueprints/BPI_Interactable.BPI_Interactable_C"))))